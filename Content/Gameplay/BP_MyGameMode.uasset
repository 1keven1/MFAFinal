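; Game mode Blueprint that offers shared helpers for highlighting meshes and toggling the level's teleport points.
; Highlighting switches a component's custom depth with stencil value 1, either directly or for a timed period via a delayed event.
; BeginPlay caches all BP_TeleportPoint actors; ControlAllTeleportPoint re-shows only those flagged Vis, or hides all.
; The IA_Test event is empty, and its input mapping setup is unconnected.
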(event `CE_SetShiningForTime`
  (params (Comp :type "StaticMeshComponent Object Reference") (Time :type "Float (double-precision)"))
  (`self.SetShining` Comp true)
  (`KismetSystemLibrary.Delay` Time)
  (`self.SetShining` Comp))

(event `self.ReceiveBeginPlay`
  (`|ExecutionSequence`
    (:`then_1`
      (bind _outactors (`GameplayStatics.GetAllActorsOfClass` "/Game/Gameplay/BP_TeleportPoint.BP_TeleportPoint_C"))
      (set `self.TeleportPoints` _outactors))))

(event `EnhancedInput|/Game/Gameplay/MyInput/IA_Test`
  (params (ActionValue :type Boolean) (ElapsedSeconds :type "Float (double-precision)") (TriggeredSeconds :type "Float (double-precision)") (InputAction :type "InputAction Object Reference" :default "/Game/Gameplay/MyInput/IA_Test.IA_Test")))

(fn `ControlAllTeleportPoint`
  (params (bEnable :type Boolean))
  (bind _teleportpoints (`self.TeleportPoints`))
  (if bEnable
    (for _array_element _teleportpoints
      (if (`/Game/Gameplay/BP_TeleportPoint.bVis` _array_element)
        (`/Game/Gameplay/BP_TeleportPoint.ChangeVis` _array_element true)))
    (else
      (for _array_element_2 _teleportpoints
        (`/Game/Gameplay/BP_TeleportPoint.ChangeVis` _array_element_2 false)))))

(fn `SetShining`
  (params (SMComp :type "StaticMeshComponent Object Reference") (bShine :type Boolean))
  (`PrimitiveComponent.SetRenderCustomDepth` SMComp bShine)
  (`PrimitiveComponent.SetCustomDepthStencilValue` SMComp 1))

(fn `UserConstructionScript`)
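; BP_TeleportPoint is a teleport destination with a Niagara ring that reflects whether it is selected.
; When a pawn teleports in, the point hides, disables collision, binds to that pawn's teleport dispatcher and fires its own.
; When the pawn's dispatcher fires, TeleportGo restores visibility and collision, then unbinds, so the point stays hidden only until that event.
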(event `CE_ChangeSelectState`
  (params (bSelect :type Boolean))
  (`NiagaraComponent.SetVariableBool` (`self.NS_MyTeleportRing`) "bSelected" bSelect))

(event `CE_TeleportCome`
  (params (Pawn :type "/Game/Gameplay/BP_MyVRPawn Object Reference"))
  (`self.ChangeVis` false)
  (set `self.bVis` false)
  (add `/Game/Gameplay/BP_MyVRPawn.ED_Teleport` Pawn (delegate `TeleportGo`))
  (`self.ED_Teleport`))

(event `TeleportGo`
  (`self.ChangeVis` true)
  (set `self.bVis` true)
  (remove `/Game/Gameplay/BP_MyVRPawn.ED_Teleport` (stale `CE_TeleportCome` Pawn) (delegate `TeleportGo`)))

(fn `ChangeVis`
  (params (bVis :type Boolean))
  (`self.SetActorHiddenInGame` (not bVis))
  (`self.SetActorEnableCollision` bVis))

(fn `UserConstructionScript`)
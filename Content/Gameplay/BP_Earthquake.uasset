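; BP_Earthquake simulates an earthquake by shaking a list of actors around the locations cached at BeginPlay.
; A shake timeline offsets each actor by transverse intensity on X/Y and longitudinal intensity on Z, scaled by a fade value.
; Start and stop events play or reverse a timed fade timeline, which also scales shake play rate and stops shaking once faded out.
; SetFrequencyAndIntensity updates both wave intensities and the frequency.
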(event `self.ReceiveBeginPlay`
  (`|ExecutionSequence`
    (:`then_0`
      (for _array_element (`self.Actors`)
        (`KismetArrayLibrary.Array_Add` (`self.ActorInitPos`) (`self.K2_GetActorLocation` _array_element))))
    (:`then_1`
      (`TimelineComponent.SetPlayRate` (`self.TL_Earthquake`) (`self.Frequency`)))))

(event `CE_StartShake`
  (params (FadeInTime :type "Float (double-precision)" :default 1.0))
  (bind _tl_fadeinout (`self.TL_FadeInOut`))
  (`TimelineComponent.SetPlayRate` _tl_fadeinout (/ 1.0 FadeInTime))
  (`TimelineComponent.Play` _tl_fadeinout)
  (`TimelineComponent.Play` (`self.TL_Earthquake`)))

(event `CE_StopShake`
  (params (FadeOutTime :type "Float (double-precision)" :default 1.0))
  (bind _tl_fadeinout (`self.TL_FadeInOut`))
  (`TimelineComponent.SetPlayRate` _tl_fadeinout (/ 1.0 FadeOutTime))
  (`TimelineComponent.Reverse` _tl_fadeinout))

(fn `SetFrequencyAndIntensity`
  (params (TransversWaveIntensity :type "Float (double-precision)") (LongitudinalWaveIntensity :type "Float (double-precision)") (Frequency :type "Float (double-precision)"))
  (`|ExecutionSequence`
    (:`then_0`
      (set `self.TransversWaveIntensity` TransversWaveIntensity)
      (set `self.LongitudinalWaveIntensity` LongitudinalWaveIntensity))
    (:`then_1`
      (bind _output_get (set `self.Frequency` Frequency))
      (`TimelineComponent.SetPlayRate` (`self.TL_Earthquake`) _output_get))))

(fn `UserConstructionScript`)
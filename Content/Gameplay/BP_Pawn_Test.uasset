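; BP_Pawn_Test is a test pawn with input-driven look and mouse-aimed teleporting between BP_TeleportPoint actors.
; A camera-channel trace from the deprojected mouse position tracks and highlights the aimed point on move input or teleport press.
; Releasing teleport moves the pawn to that point's X/Y, keeps its height, fires the teleport dispatcher and clears the highlight.
; The point's CETeleportCome notification is unwired.
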(event `self.ReceiveBeginPlay`
  (set `self.MyController` (cast `PlayerController` (`self.GetController`) :!pure true)))

(event `EnhancedInput|/Game/Gameplay/MyInput/IA_Test_Turn`
  (params (ActionValue :type "Vector2D Structure") (ElapsedSeconds :type "Float (double-precision)") (TriggeredSeconds :type "Float (double-precision)") (InputAction :type "InputAction Object Reference" :default "/Game/Gameplay/MyInput/IA_Test_Turn.IA_Test_Turn"))
  (bind _returnvalue (`GameplayStatics.GetPlayerController` 0))
  (bind (_x _y) (`KismetMathLibrary.BreakVector2D` ActionValue))
  (:`Triggered`
    (`PlayerController.AddPitchInput` _returnvalue _y)
    (`PlayerController.AddYawInput` _returnvalue _x)))

(event `EnhancedInput|/Game/Gameplay/MyInput/IA_Test_TeleportMove`
  (params (ActionValue :type "Vector2D Structure") (ElapsedSeconds :type "Float (double-precision)") (TriggeredSeconds :type "Float (double-precision)") (InputAction :type "InputAction Object Reference" :default "/Game/Gameplay/MyInput/IA_Test_TeleportMove.IA_Test_TeleportMove"))
  (bind _aimedteleport (`self.AimedTeleport`))
  (bind (_worldlocation _worlddirection) (`PlayerController.DeprojectMousePositionToWorld` (`self.MyController`)))
  (:`Triggered`
    (bind (_outhit _returnvalue) (`KismetSystemLibrary.LineTraceSingle` :`Start` _worldlocation :`End` (+ _worldlocation (* _worlddirection 1000)) :`TraceChannel` "TraceTypeQuery2" :`DrawTime` 2.0 :!label _label))
    (if _returnvalue
      (bind _asbp_teleport_point (cast `/Game/Gameplay/BP_TeleportPoint` (`.HitActor` (`GameplayStatics.BreakHitResult` _outhit)))
        (:`then`
          (bind _output_get (set `self.AimedTeleport` _asbp_teleport_point))
          (`/Game/Gameplay/BP_TeleportPoint.CE_ChangeSelectState` _output_get true))
        (:`CastFailed`
          (`/Engine/EditorBlueprintResources/StandardMacros.IsValid` _aimedteleport :!label _label_2
            (:`Is Valid`
              (`/Game/Gameplay/BP_TeleportPoint.CE_ChangeSelectState` _aimedteleport false)
              (set `self.AimedTeleport` null)))))
      (else
        (goto _label_2)))))

(event `EnhancedInput|/Game/Gameplay/MyInput/IA_Test_Teleport`
  (params (ActionValue :type Boolean) (ElapsedSeconds :type "Float (double-precision)") (TriggeredSeconds :type "Float (double-precision)") (InputAction :type "InputAction Object Reference" :default "/Game/Gameplay/MyInput/IA_Test_Teleport.IA_Test_Teleport"))
  (:`Triggered`
    (if ActionValue
      (if (not (`self.bShowTeleportLine`))
        (set `self.bShowTeleportLine` true)
        (goto _label))
      (else
        (set `self.bShowTeleportLine` false)
        (`self.TryTeleport` (`self.AimedTeleport`))
        (set `self.AimedTeleport` null)))))

(fn `TryTeleport`
  (params (TeleportObj :type "/Game/Gameplay/BP_TeleportPoint Object Reference (by ref)"))
  (bind (_returnvalue_x _returnvalue_y) (`KismetMathLibrary.BreakVector` (`self.K2_GetActorLocation` TeleportObj)))
  (bind (_returnvalue_x_2 _returnvalue_y_2 _returnvalue_z) (`KismetMathLibrary.BreakVector` (`self.K2_GetActorLocation`)))
  (`/Engine/EditorBlueprintResources/StandardMacros.IsValid` TeleportObj
    (:`Is Valid`
      (`|ExecutionSequence`
        (:`then_0`
          (`self.K2_SetActorLocation` (`KismetMathLibrary.MakeVector` _returnvalue_x _returnvalue_y _returnvalue_z))
          (`self.ED_Teleport`))
        (:`then_1`
          (`/Game/Gameplay/BP_TeleportPoint.CE_ChangeSelectState` TeleportObj false))))))

(fn `UserConstructionScript`)